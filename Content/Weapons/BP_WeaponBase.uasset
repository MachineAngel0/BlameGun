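; BP_WeaponBase is a base weapon actor that characters pick up by overlapping its sphere.
; On overlap it requests the character via a message, then registers itself as CurrentWeapon on that character's EquipWeaponComponent.
; It snaps the skeletal mesh to the GripPoint socket and sets HasRifle on the FirstPerson_AnimBP.
; BeginPlay prints the names of its WeaponBaseComponent components for debugging.
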(event OnComponentBeginOverlap(Sphere)
  (params (OverlappedComponent :type Primitive%20Component%20Object%20Reference) (OtherActor :type Actor%20Object%20Reference) (OtherComp :type Primitive%20Component%20Object%20Reference) (OtherBodyIndex :type Integer) (bFromSweep :type Boolean) (SweepResult :type Hit%20Result%20Structure%20%28by%20ref%29))
  (bind _returnvalue (Class|InterfaceCharacter|RequestCharacter(Message) OtherActor))
  (Utilities|IsValid _returnvalue
    (:Is%20Valid
      (Utilities|IsValid (Actor|GetComponentbyClass _returnvalue "/Script/BlameGun.EquipWeaponComponent")
        (:Is%20Valid
          (Variables|/Script/BlameGun.EquipWeaponComponent|SetCurrentWeapon (Actor|GetComponentbyClass _returnvalue "/Script/BlameGun.EquipWeaponComponent") self)
          (Transformation|AttachComponentToComponent (Variables|Default|GetWeaponSkeletalMesh) (Class|CharacterBase|GetCharacterMesh _returnvalue) "GripPoint" "SnapToTarget" "SnapToTarget" "SnapToTarget" true)
          (bind _asfirst_person_anim_bp (Utilities|Casting|CastToFirstPerson_AnimBP (Components|SkeletalMesh|GetAnimInstance (Class|CharacterBase|GetCharacterMesh _returnvalue))))
          (Variables|/Game/FirstPersonArms/Animations/FirstPerson_AnimBP.FirstPerson_AnimBP_C|SetHasRifle _asfirst_person_anim_bp true))))))

(event EventBeginPlay
  (for _array_element (Actor|GetComponentsByClass self "/Script/BlameGun.WeaponBaseComponent")
    (Development|PrintString (Utilities|GetDisplayName _array_element) true true "(R=1.000000,G=0.233938,B=0.000000,A=1.000000)" 5e+01)))

(event Collision|EventActorBeginOverlap
  (params (OtherActor :type Actor%20Object%20Reference)))

(event EventTick
  (params (DeltaSeconds :type Float%20%28single-precision%29)))

(fn ConstructionScript)