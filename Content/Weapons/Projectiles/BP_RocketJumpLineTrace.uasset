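; One-shot rocket jump projectile actor that hitscans from the player camera and applies a radial impulse at the point it hits.
; On BeginPlay it sets the RadialForce radius and strength from one of five TestNumber tuning presets, then runs a long Visibility trace.
; A hit moves the force to the impact, fires it, spawns VFX and draws debug radius.
; The actor destroys itself whether or not it hits.
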(event Custom|InitRadialForce
  (bind _radialforce (Variables|Default|GetRadialForce))
  (bind _radialforce_2 (Variables|Default|GetRadialForce))
  (bind _radialforce_3 (Variables|Default|GetRadialForce))
  (bind _radialforce_4 (Variables|Default|GetRadialForce))
  (bind _radialforce_5 (Variables|Default|GetRadialForce))
  (switch Utilities|FlowControl|Switch|SwitchonETestNumber (Variables|Default|GetTestNumber)
    (:ECS_Test1
      (Variables|/Script/Engine.RadialForceComponent|SetRadius _radialforce_5 (Variables|Default|GetRadius_1))
      (Variables|/Script/Engine.RadialForceComponent|SetImpulseStrength _radialforce_5 (Variables|Default|GetImpulseStrength_1)))
    (:ECS_Test2
      ;[0.15 0.15 0.15 0.5] tiny radius, extreme force
      (Variables|/Script/Engine.RadialForceComponent|SetRadius _radialforce (Variables|Default|GetRadius_2))
      (Variables|/Script/Engine.RadialForceComponent|SetImpulseStrength _radialforce (Variables|Default|GetImpulseStrength_2)))
    (:ECS_Test3
      ;[0.15 0.15 0.15 0.5] Large Radius tiny force
      (Variables|/Script/Engine.RadialForceComponent|SetRadius _radialforce_2 (Variables|Default|GetRadius_3))
      (Variables|/Script/Engine.RadialForceComponent|SetImpulseStrength _radialforce_2 (Variables|Default|GetImpulseStrength_3)))
    (:ECS_Test4
      ;[0.15 0.15 0.15 0.5] Extreme radius tiny force
      (Variables|/Script/Engine.RadialForceComponent|SetRadius _radialforce_4 (Variables|Default|GetRadius_4))
      (Variables|/Script/Engine.RadialForceComponent|SetImpulseStrength _radialforce_4 (Variables|Default|GetImpulseStrength_4)))
    (:ECS_Test5
      ;[0.15 0.15 0.15 0.5] Large Radius tiny force
      (Variables|/Script/Engine.RadialForceComponent|SetRadius _radialforce_3 (Variables|Default|GetRadius_5))
      (Variables|/Script/Engine.RadialForceComponent|SetImpulseStrength _radialforce_3 (Variables|Default|GetImpulseStrength_5)))))

(event EventBeginPlay
  (bind _returnvalue (Game|GetPlayerCameraManager 0))
  (bind _radialforce (Variables|Default|GetRadialForce))
  (CallFunction|InitRadialForce)
  (bind (_outhit _returnvalue_2) (Collision|LineTraceByChannel (Transformation|GetWorldLocation (Variables|/Script/Engine.Actor|GetRootComponent _returnvalue)) (+ (* (Math|Vector|GetForwardVector (Variables|/Script/Engine.Actor|GetRootComponent _returnvalue)) 5e+04) (Transformation|GetActorLocation _returnvalue)) "TraceTypeQuery1" false 0 "ForDuration"))
  (if _returnvalue_2
    (Transformation|SetWorldLocation _radialforce (.ImpactPoint (Collision|BreakHitResult _outhit)) false true)
    (Class|RadialForceComponent|FireImpulse _radialforce)
    (Default|SpawnVFX (Variables|Default|GetBPC_VFXSpawner) (.ImpactPoint (Collision|BreakHitResult _outhit)) "0, 0, 0")
    (Rendering|Debug|DrawDebugSphere (.ImpactPoint (Collision|BreakHitResult _outhit)) (Variables|/Script/Engine.RadialForceComponent|GetRadius (Variables|Default|GetRadialForce)) 12 "(R=1.000000,G=0.000000,B=0.070807,A=1.000000)" 5.0)
    (Actor|DestroyActor)
    (else
      (Actor|DestroyActor))))

(event Collision|EventActorBeginOverlap
  (params (OtherActor :type Actor%20Object%20Reference)))

(fn ConstructionScript)